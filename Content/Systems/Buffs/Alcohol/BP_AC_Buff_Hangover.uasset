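; Hangover buff component from the alcohol buff set, described to the player as reduced maximum stamina and slightly faster thirst.
; Its start, tick and clear events are empty; the logic for the StaminaMax modifier and hunger-system drink drain sits in disconnected nodes that never run.
; Only the effect description is functional in this graph, formatting the MaxStaminaPenalty value into its text.
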(event EventStartBuff
  (params (BuffPotency :type Integer) (OwningCharacter :type Conan%20Character%20Object%20Reference) (Instigator :type Controller%20Object%20Reference)))

(event EventGameplayEffecttoApplyonBuffStart)

(event EventGameplayEffecttoApplyonBuffCleared)

(event EventGameplayEffecttoApplyonBuffTick)

(fn GetEffectDescription
  (return (Utilities|Text|FormatText "Maximum Stamina reduced  by {StaminaMaxReduction}. Thirst rate slightly increased." (Variables|Default|GetMaxStaminaPenalty))))