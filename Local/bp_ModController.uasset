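; Mod controller that tones down mature content (rude text, revealing armour, slavery, cannibalism, evil religions) and adjusts resource harvesting through data table edits.
; ModDataTableOperations merges FF_ override tables into game tables for items, feats, armour, loot, resources, religions, dialogue and spawns.
; It also deletes slavery feat and cannibal recipe rows by ID.
; An unused ItemTable removal stays disconnected because removing the feats that grant those recipes suffices.
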(event EventBeginPlay)

(event EventTick
  (params (DeltaSeconds :type Float%20%28single-precision%29)))

(fn ConstructionScript)

(fn ModDataTableOperations
  (Class|ModController|MergeDataTables "/Game/Items/ItemTable.ItemTable" "/Game/Mods/FamilyFriendly/DataTables/FF_dt_RudeTextItems.FF_dt_RudeTextItems") ; Remove rude words from some item descriptions.
  (Class|ModController|RemoveDataTableRows "/Game/Items/Feats/FeatTable.FeatTable" (Utilities|Array|MakeArray "51961" "89912" "89913")) ; Remove slavery-related feats.
  (Class|ModController|MergeDataTables "/Game/Items/Feats/FeatTable.FeatTable" "/Game/Mods/FamilyFriendly/DataTables/FF_dt_Feats.FF_dt_Feats")
  (Class|ModController|MergeDataTables "/Game/Items/EquipmentVariationTable.EquipmentVariationTable" "/Game/Mods/FamilyFriendly/DataTables/FF_dt_RudeArmour.FF_dt_RudeArmour") ; Change some revealing armour models to more modest alternatives.
  (Class|ModController|MergeDataTables "/Game/Systems/Survival/Gathering/Gathering_v2/LootTable_Resource.LootTable_Resource" "/Game/Mods/FamilyFriendly/DataTables/Gathering/FF_dt_LootTableResource.FF_dt_LootTableResource")
  (Class|ModController|MergeDataTables "/Game/Systems/Survival/Gathering/Gathering_v2/ResourceLootTemplates.ResourceLootTemplates" "/Game/Mods/FamilyFriendly/DataTables/Gathering/FF_dt_ResourceLootTemplates.FF_dt_ResourceLootTemplates")
  (Class|ModController|MergeDataTables "/Game/Systems/Survival/Gathering/Gathering_v2/ResourceStatTable.ResourceStatTable" "/Game/Mods/FamilyFriendly/DataTables/Gathering/FF_dt_ResourceStat.FF_dt_ResourceStat") ; Make some harvested resources 'exclusive' so they can only appear when using thier dedicated harvesting tool.
  (Class|ModController|MergeDataTables "/Game/Systems/Survival/Gathering/Gathering_v2/WeaponTypeResourceStatTable.WeaponTypeResourceStatTable" "/Game/Mods/FamilyFriendly/DataTables/Gathering/FF_dt_WeaponTypeResource.FF_dt_WeaponTypeResource") ; Change what type of resources can be harvested by different harvesting tools.
  (Class|ModController|RemoveDataTableRows "/Game/Items/Recipes/RecipesTable.RecipesTable" (Utilities|Array|MakeArray "12010" "12011" "13053" "18270" "19902")) ; Remove some cannibalistic recipes.
  (Class|ModController|MergeDataTables "/Game/UI/CharacterCreation/DataTables/ReligionSelections.ReligionSelections" "/Game/Mods/FamilyFriendly/DataTables/FF_dt_ReligionSelect.FF_dt_ReligionSelect")
  (Class|ModController|MergeDataTables "/Game/Systems/Dialogue/NpcDialogues.NpcDialogues" "/Game/Mods/FamilyFriendly/DataTables/FF_dt_NPCDialogues.FF_dt_NPCDialogues") ; Prevent learning evil religions from NPCs.
  (Class|ModController|MergeDataTables "/Game/Systems/SpawnTable/SpawnDataTable.SpawnDataTable" "/Game/Mods/FamilyFriendly/DataTables/FF_dt_Thralls.FF_dt_Thralls"))